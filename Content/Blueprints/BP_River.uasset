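; BP_River is a river actor that carries BP_Prop objects along with its current and recycles them to their spawn points.
; River hits register props and set every registered prop's velocity along the Arrow's direction; character hits only store a player reference.
; On Box overlap, a prop loses physics while a Timeline sinks it, moves it below its spawn location, then reverses to raise it before restoring physics.
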(event `self.River.OnComponentHit`
  (params (HitComponent :type "PrimitiveComponent Object Reference") (OtherActor :type "Actor Object Reference") (OtherComp :type "PrimitiveComponent Object Reference") (NormalImpulse :type "Vector Structure") (Hit :type "HitResult Structure (by ref)"))
  (bind (_bblockinghit _binitialoverlap _time _distance _location _impactpoint _normal _impactnormal _physmat _hitactor) (`GameplayStatics.BreakHitResult` Hit))
  (if (`KismetMathLibrary.ClassIsChildOf` (`GameplayStatics.GetObjectClass` _hitactor) "/Game/Blueprints/BP_Prop.BP_Prop_C")
    (bind _asbp_prop (cast `/Game/Blueprints/BP_Prop` _hitactor))
    (`/Game/Blueprints/BP_Prop.Initialize` _asbp_prop)
    (`KismetArrayLibrary.Array_AddUnique` (`self.Props`) _asbp_prop)
    (`self.Launch Props`)
    (elif (`KismetMathLibrary.ClassIsChildOf` (`GameplayStatics.GetObjectClass` OtherActor) "/Game/Blueprints/Character/BP_ThirdPersonCharacter.BP_ThirdPersonCharacter_C")
      (bind _asbp_third_person_character (cast `/Game/Blueprints/Character/BP_ThirdPersonCharacter` OtherActor))
      (set `self.PlayerRef` _asbp_third_person_character))))

(event `self.Box.OnComponentBeginOverlap`
  (params (OverlappedComponent :type "PrimitiveComponent Object Reference") (OtherActor :type "Actor Object Reference") (OtherComp :type "PrimitiveComponent Object Reference") (OtherBodyIndex :type Integer) (bFromSweep :type Boolean) (SweepResult :type "HitResult Structure (by ref)"))
  (bind _asbp_prop (cast `/Game/Blueprints/BP_Prop` OtherActor))
  (bind _staticmesh (`/Game/Blueprints/BP_Prop.StaticMesh` _asbp_prop))
  (`/Engine/EditorBlueprintResources/StandardMacros.IsValid` _staticmesh
    (:`Is Valid`
      (bind _staticmesh_2 (`/Game/Blueprints/BP_Prop.StaticMesh` _asbp_prop))
      (`PrimitiveComponent.SetEnableGravity` _staticmesh_2 false)
      (`PrimitiveComponent.SetSimulatePhysics` _staticmesh_2 false)
      (bind (_direction _newtrack_0) (`Timeline|Timeline` :!label _label)
        (:`Update`
          (bind (_returnvalue_x _returnvalue_y) (`KismetMathLibrary.BreakVector` (`SceneComponent.K2_GetComponentLocation` _staticmesh)))
          (bind (_spawnlocation_x _spawnlocation_y _spawnlocation_z) (`KismetMathLibrary.BreakVector` (`/Game/Blueprints/BP_Prop.SpawnLocation` _asbp_prop)))
          (`SceneComponent.K2_SetWorldLocation` _staticmesh (`KismetMathLibrary.VLerp` (`KismetMathLibrary.MakeVector` _returnvalue_x _returnvalue_y _spawnlocation_z) (`KismetMathLibrary.MakeVector` _returnvalue_x _returnvalue_y (- _spawnlocation_z 150.0)) _newtrack_0) false false))
        (:`Finished`
          (switch `ETimelineDirection` _direction
            (:`Forward`
              (`SceneComponent.K2_SetWorldLocation` _staticmesh (- (`/Game/Blueprints/BP_Prop.SpawnLocation` _asbp_prop) (0.0 0.0 150.0)) false false)
              (goto _label :!via `Reverse`))
            (:`Backward`
              (bind _staticmesh_3 (`/Game/Blueprints/BP_Prop.StaticMesh` _asbp_prop))
              (`PrimitiveComponent.SetEnableGravity` _staticmesh_3 true)
              (`PrimitiveComponent.SetSimulatePhysics` _staticmesh_3 true))))))))

(event `Launch Props`
  ;[0 0.09409 1 1 39] Add velocity to Props
  (for _array_element (`self.Props`)
    (`PrimitiveComponent.SetPhysicsLinearVelocity` (`/Game/Blueprints/BP_Prop.StaticMesh` _array_element) (* (`KismetMathLibrary.GetForwardVector` (`SceneComponent.K2_GetComponentRotation` (`self.Arrow`))) 300.0) false "None")))

(fn `UserConstructionScript`)