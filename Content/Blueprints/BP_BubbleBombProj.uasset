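; BP_BubbleBombProj is a physics bubble projectile that sticks to cobwebs and inflates.
; On hitting a BP_Cobweb it stops simulating physics, starts blocking pawns, and once plays a grow sound while a timeline scales it up tenfold.
; Any other hit destroys it, except contact with the player pawn before it has stuck.
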(event `self.Bubble.OnComponentHit`
  (params (HitComponent :type "PrimitiveComponent Object Reference") (OtherActor :type "Actor Object Reference") (OtherComp :type "PrimitiveComponent Object Reference") (NormalImpulse :type "Vector Structure") (Hit :type "HitResult Structure (by ref)"))
  (bind (_bblockinghit _binitialoverlap _time _distance _location _impactpoint _normal _impactnormal _physmat _hitactor) (`GameplayStatics.BreakHitResult` Hit))
  (bind _bubble (`self.Bubble`))
  (if (not (`KismetMathLibrary.ClassIsChildOf` (`GameplayStatics.GetObjectClass` _hitactor) "/Game/Blueprints/BP_Cobweb.BP_Cobweb_C"))
    (if (not (and (not (`self.isSticked`)) (== _hitactor (`GameplayStatics.GetPlayerPawn` 0))))
      (`self.K2_DestroyActor`))
    (else
      (`PrimitiveComponent.SetPhysicsLinearVelocity` (`self.Bubble`) (0.0 0.0 0.0) false "None")
      (`PrimitiveComponent.SetCollisionResponseToChannel` _bubble "ECC_Pawn" "ECR_Block")
      (set `self.isSticked` true)
      (`PrimitiveComponent.SetSimulatePhysics` _bubble false)
      (`/Engine/EditorBlueprintResources/StandardMacros.DoOnce` false
        (:`Completed`
          (set `self.isSticked` true)
          (`GameplayStatics.PlaySound2D` "/Game/Sounds/SW_GrowBubble.SW_GrowBubble" 1.0 1.0 0.0 null null)
          (bind (_direction _alpha) (`Timeline|Timeline` :!via `PlayFromStart`)
            (:`Update`
              (`SceneComponent.SetWorldScale3D` (`self.Bubble`) (`KismetMathLibrary.VLerp` (0.2 0.2 0.2) (2.0 2.0 2.0) _alpha)))))))))

(fn `UserConstructionScript`)